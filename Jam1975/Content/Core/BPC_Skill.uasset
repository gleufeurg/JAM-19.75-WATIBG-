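; BPC_Skill is a component that tracks the cooldown of a skill.
; While the skill is uncharged, Tick adds world delta seconds to a timer until it reaches the CDSkill duration, then flags it as charged.
; BeginPlay starts the skill uncharged, and UseSkill resets the timer and flag without checking charge or running any skill effect.
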(event `self.ReceiveBeginPlay`
  (set `self.TimeBeforeCharge` 0.0)
  (set `self.isCharged` false))

(event `Use Skill`
  (set `self.isCharged` false)
  (set `self.TimeBeforeCharge` 0.0))

(event `CoolDown SKill`
  (if (< (`self.TimeBeforeCharge`) (`self.CDSkill`))
    (set `self.TimeBeforeCharge` (+ (`self.TimeBeforeCharge`) (`GameplayStatics.GetWorldDeltaSeconds`)))
    (else
      (set `self.isCharged` true))))

(event `self.ReceiveTick`
  (params (DeltaSeconds :type "Float (single-precision)"))
  (if (not (`self.isCharged`))
    (`self.CoolDown SKill`)))