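; Sound manager actor that plays the ambient and Hell background loops and positional effects for dimension travel, doors, spikes and damage.
; BeginPlay creates both 2D sounds and starts the ambient one; Hell audio first plays on entering the dimension, guarded by a DoOnce.
; Entering or leaving the dimension calls Transition, which crossfades the ambient and Hell sound classes through sound mix class overrides.
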(event `self.ReceiveBeginPlay`
  (bind _returnvalue (`GameplayStatics.CreateSound2D` "/Game/Core/Sound/Sound/Ambient_cue.Ambient_cue" 1.0 1.0 0.0 null false false))
  (set `self.Ambient_sound` _returnvalue)
  (bind _returnvalue_2 (`GameplayStatics.CreateSound2D` "/Game/Core/Sound/Sound/Hell_cue.Hell_cue" 1.0 1.0 0.0 null false false))
  (set `self.Hell_sound` _returnvalue_2)
  (`AudioComponent.Play` (`self.Ambient_sound`) 0.0))

(event `InDimension`
  (params (Location :type "Vector Structure"))
  (`GameplayStatics.PlaySoundAtLocation` "/Game/Core/Sound/Sound/EnteringDimension_Cue.EnteringDimension_Cue" Location (struct) 1.0 1.0 0.0 "/Game/Core/Sound/SA_generic.SA_generic" null null null)
  (`self.Transition` "/Game/Core/Sound/SC_ambient.SC_ambient" "/Game/Core/Sound/SC_Hell.SC_Hell" 0.3)
  (`/Engine/EditorBlueprintResources/StandardMacros.DoOnce` false
    (:`Completed`
      (`AudioComponent.Play` (`self.Hell_sound`) 0.0))))

(event `Spawn_door`
  (params (Location :type "Vector Structure"))
  (`GameplayStatics.PlaySoundAtLocation` "/Game/Core/Sound/Sound/Open_door_sound_Cue.Open_door_sound_Cue" Location (struct) 1.0 1.0 0.0 "/Game/Core/Sound/SA_generic.SA_generic" null null null))

(event `OutDimension`
  (params (Location :type "Vector Structure"))
  (`GameplayStatics.PlaySoundAtLocation` "/Game/Core/Sound/Sound/Crack_sound_Cue.Crack_sound_Cue" Location (struct) 1.0 1.0 0.0 "/Game/Core/Sound/SA_generic.SA_generic" null null null)
  (`self.Transition` "/Game/Core/Sound/SC_Hell.SC_Hell" "/Game/Core/Sound/SC_ambient.SC_ambient" 0.3))

(event `Spikes`
  (params (Location :type "Vector Structure"))
  (`GameplayStatics.PlaySoundAtLocation` "/Game/Core/Sound/Sound/Spikes_sound_Cue.Spikes_sound_Cue" Location (struct) 1.0 1.0 0.0 "/Game/Core/Sound/SA_generic.SA_generic" null null null))

(event `Damage_sound`
  (params (Location :type "Vector Structure"))
  (`GameplayStatics.PlaySoundAtLocation` "/Game/Core/Sound/Sound/Damage_sound_Cue.Damage_sound_Cue" Location (struct) 1.0 1.0 0.0 "/Game/Core/Sound/SA_generic.SA_generic" null null null))

(fn `UserConstructionScript`)