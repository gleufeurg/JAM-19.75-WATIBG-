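; AI pawn that moves between linked target points, diverts to walls it spots, and ragdolls on death.
; A repeating AIMoveTo picks random or sequential points, while Focus holds the wall until it becomes invalid, then restores the previous target and usual behaviour.
; Each tick, a forward sphere trace sized by PawnSensing values looks for BP_Wall.
; Lethal damage enables physics and has the passed PhysicsHandle grab the hit bone.
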(event `self.ReceiveTick`
  (params (DeltaSeconds :type "Float (single-precision)"))
  (`self.Search for Objects`))

(event `self.ReceiveBeginPlay`
  (set `self.Choose Destination Behaviour` (`self.Usual Behaviour`))
  (`self.Move to Point`))

(event `Move to Point`
  (`self.Choose Destination` :!label _label)
  (`|AIMoveTo` self (0.0 0.0 0.0) (`self.Target_point`) 10.0
    (:`OnSuccess`
      (goto _label))))

(event `Search for Objects`
  (bind _returnvalue (`self.K2_GetActorLocation`))
  (bind _pawnsensing (`self.PawnSensing`))
  (bind _outhit (`KismetSystemLibrary.SphereTraceSingle` _returnvalue (+ _returnvalue (* (`self.GetActorForwardVector`) (`PawnSensingComponent.SightRadius` _pawnsensing))) (`PawnSensingComponent.PeripheralVisionAngle` _pawnsensing) "TraceTypeQuery1"))
  (bind (_bblockinghit _binitialoverlap _time _distance _location _impactpoint _normal _impactnormal _physmat _hitactor) (`GameplayStatics.BreakHitResult` _outhit))
  (if (== (`GameplayStatics.GetObjectClass` _hitactor) "/Game/Skills/Wall/BP_Wall.BP_Wall_C")
    (set `self.Choose Destination Behaviour` "NewEnumerator2")
    (set `self.Target_point` _hitactor) ; Must have target points linked in the scene
    (`self.Move to Point`)))

(event `Choose Destination`
  (bind _list_run_away_point (`self.List_run_away_point`))
  (bind _target_count (`self.Target Count`))
  (switch `/Game/IA/EAIDestinationBehavior` (`self.Choose Destination Behaviour`) ; predefined, not available for now
    (:`NewEnumerator0`
      (set `self.Previous Target Point` (`self.Target_point`))
      (set `self.Target_point` (`KismetArrayLibrary.Array_Random` (`self.List_run_away_point`))) ; Must have target points linked in the scene
    )
    (:`NewEnumerator1`
      (set `self.Previous Target Point` (`self.Target_point`))
      (set `self.Target_point` (`|GetArrayItem` _list_run_away_point _target_count)) ; Must have target points linked in the scene
      (set `self.Target Count` (mod (+ 1 _target_count) (- (`KismetArrayLibrary.Array_Length` _list_run_away_point) 1))))
    (:`NewEnumerator2`
      (`/Engine/EditorBlueprintResources/StandardMacros.IsValid` (`self.Target_point`)
        (:`Is Not Valid`
          (set `self.Choose Destination Behaviour` (`self.Usual Behaviour`))
          (set `self.Target_point` (`self.Previous Target Point`)))))))

(event `/Game/IA/ITakeDamage.Take Damage`
  (params (Damage :type "Float (double-precision)") (`Bone Hit` :type Name) (`Hit Component` :type "PrimitiveComponent Object Reference") (`Impact Point` :type "Vector Structure") (Physic :type "ActorComponent Object Reference"))
  (set `self.Life` (- (`self.Life`) Damage))
  (if (<= (`self.Life`) 0.0)
    (`self.Die`)))

(event `Die`
  (`PrimitiveComponent.SetSimulatePhysics` (`self.Mesh`) true)
  (`PhysicsHandleComponent.GrabComponentAtLocation` (cast `PhysicsHandleComponent` (stale `/Game/IA/ITakeDamage.Take Damage` Physic) :!pure true) (stale `/Game/IA/ITakeDamage.Take Damage` `Hit Component`) (stale `/Game/IA/ITakeDamage.Take Damage` `Bone Hit`) (stale `/Game/IA/ITakeDamage.Take Damage` `Impact Point`))
  (`PrimitiveComponent.SetCollisionObjectType` (`self.Mesh`) "ECC_PhysicsBody")
  (`PrimitiveComponent.SetCollisionEnabled` (`self.CapsuleComponent`) "NoCollision"))

(event `Upd`
  (`/Engine/EditorBlueprintResources/StandardMacros.IsValid` (stale `/Game/IA/ITakeDamage.Take Damage` `Hit Component`)
    (:`Is Valid`
      (`PhysicsHandleComponent.SetTargetLocation` (cast `PhysicsHandleComponent` (stale `/Game/IA/ITakeDamage.Take Damage` Physic) :!pure true) (stale `/Game/IA/ITakeDamage.Take Damage` `Impact Point`))
      (`KismetSystemLibrary.Delay` 0.01)
      (`self.Upd`))))

(fn `UserConstructionScript`)