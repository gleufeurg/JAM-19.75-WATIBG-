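; Dimension door actor that switches the world's look and gives the first-person character dimension movement when a Character enters its box.
; Tick eases the medieval door mesh open by 90 degrees of yaw from its starting rotation, independent of the overlap.
; The construction script copies settings from the first "Dimension"-tagged PostProcessVolume into its own post process.
; Entering the box makes that post process unbound; leaving reverts nothing.
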(event `self.ReceiveBeginPlay`
  (set `self.Relative Rotation` (`SceneComponent.RelativeRotation` (`self.MedievalDoor_FBX`))))

(event `self.ReceiveTick`
  (params (DeltaSeconds :type "Float (single-precision)"))
  (bind _relative_rotation (`self.Relative Rotation`))
  (bind _medievaldoor_fbx (`self.MedievalDoor_FBX`))
  (bind _returnvalue (`KismetMathLibrary.MakeRotator` (.roll _relative_rotation) (.pitch _relative_rotation) (+ (.yaw _relative_rotation) -90.0)))
  (if (not (<= (.yaw (`SceneComponent.RelativeRotation` _medievaldoor_fbx)) (.yaw _returnvalue)))
    (set `self.Alpha` (+ (`GameplayStatics.GetWorldDeltaSeconds`) (`self.Alpha`) 0.0))
    (`SceneComponent.K2_SetRelativeRotation` _medievaldoor_fbx (`|EaseFunction` "EaseIn" (`self.Alpha`) _relative_rotation _returnvalue false 0.15) false false)))

(event `self.Box.OnComponentBeginOverlap`
  (params (OverlappedComponent :type "PrimitiveComponent Object Reference") (OtherActor :type "Actor Object Reference") (OtherComp :type "PrimitiveComponent Object Reference") (OtherBodyIndex :type Integer) (bFromSweep :type Boolean) (SweepResult :type "HitResult Structure (by ref)"))
  (cast `Character` OtherActor)
  (set `PostProcessComponent.bUnbound` true (`self.PostProcess`))
  (bind _returnvalue (`GameplayStatics.GetActorOfClass` "/Game/FirstPerson/Blueprints/BP_FirstPersonCharacter.BP_FirstPersonCharacter_C"))
  (`AddComponent|NODE_AddBPC_Dimension_Movement-0` :`self` _returnvalue))

(event `self.Box.OnComponentEndOverlap`
  (params (OverlappedComponent :type "PrimitiveComponent Object Reference") (OtherActor :type "Actor Object Reference") (OtherComp :type "PrimitiveComponent Object Reference") (OtherBodyIndex :type Integer))
  (cast `Character` OtherActor))

(fn `UserConstructionScript`
  (bind _outactors (`GameplayStatics.GetAllActorsWithTag` "Dimension"))
  (bind _output (`|GetArrayItem` _outactors))
  (`/Engine/EditorBlueprintResources/StandardMacros.IsValid` _output
    (:`Is Valid`
      (bind _aspost_process_volume (cast `PostProcessVolume` _output))
      (set `PostProcessComponent.Settings` (`PostProcessVolume.Settings` _aspost_process_volume) (`self.PostProcess`)))))