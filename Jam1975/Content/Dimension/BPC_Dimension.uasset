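; BPC_Dimension is a skill component that lets the first-person character place a dimension door in front of the camera.
; When charged, UseSkill runs the parent logic, starts the cooldown and destroys any existing BP_DimensionDoor it finds.
; It then spawns a new door a short distance along the camera's forward vector, matching camera rotation, and has BP_soundManager play its SpawnDoor event at that location.
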(event `self.Use Skill`
  (if (`self.isCharged`)
    (`parent.Use Skill`)
    (`self.CoolDown SKill`)
    (bind _asbp_first_person_character (cast `/Game/FirstPerson/Blueprints/BP_FirstPersonCharacter` (`self.GetOwner`)))
    (bind _returnvalue (`GameplayStatics.GetActorOfClass` "/Game/Dimension/BP_DimensionDoor.BP_DimensionDoor_C"))
    (`/Engine/EditorBlueprintResources/StandardMacros.IsValid` _returnvalue
      (:`Is Valid`
        (`Actor.K2_DestroyActor` _returnvalue))
      (:`Is Not Valid`
        _))
    (bind _firstpersoncamera (`/Game/FirstPerson/Blueprints/BP_FirstPersonCharacter.FirstPersonCamera` _asbp_first_person_character))
    (bind _returnvalue_2 (+ (`SceneComponent.K2_GetComponentLocation` _firstpersoncamera) (* (`SceneComponent.GetForwardVector` _firstpersoncamera) (`KismetMathLibrary.Conv_DoubleToVector` 200.0))))
    (`|SpawnActorFromClass` "/Game/Dimension/BP_DimensionDoor.BP_DimensionDoor_C" (`KismetMathLibrary.MakeTransform` _returnvalue_2 (`SceneComponent.K2_GetComponentRotation` _firstpersoncamera)) "AdjustIfPossibleButAlwaysSpawn" "MultiplyWithRoot" null null)
    (bind _returnvalue_3 (`GameplayStatics.GetActorOfClass` "/Game/Core/Sound/BP_soundManager.BP_soundManager_C"))
    (`/Game/Core/Sound/BP_soundManager.Spawn_door` _returnvalue_3 _returnvalue_2)))