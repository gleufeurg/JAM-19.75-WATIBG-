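; BP_Wall is a skill wall actor built from four cubes that plays a distance-attenuated world camera shake on BeginPlay.
; Its Fall function is written to offset a cube vertically by FallHeight, then sweep it toward a lower target with exponential easing as Alpha advances.
; The Falling event applies Fall to all four cubes, but its looping timer is disconnected, so nothing in this graph triggers the motion.
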(event `self.ReceiveBeginPlay`
  (`GameplayStatics.PlayWorldCameraShake` "/Game/FirstPerson/Blueprints/CS_wall.CS_wall_C" (`self.K2_GetActorLocation`) 500.0 3500.0))

(event `self.ReceiveTick`
  (params (DeltaSeconds :type "Float (single-precision)")))

(event `Falling`
  (bind _fall_height (`self.Fall Height`))
  (`self.Fall` (`self.Cube1`) _fall_height)
  (`self.Fall` (`self.Cube2`) _fall_height)
  (`self.Fall` (`self.Cube3`) _fall_height)
  (`self.Fall` (`self.Cube`) _fall_height))

(fn `Fall`
  (params (self2 :type "SceneComponent Object Reference") (FallHeight :type "Float (double-precision)"))
  (locals (StartSize :type "Vector Structure" :default (0.0 0.0 0.0)) (Alpha :type "Float (double-precision)") (TargetSize :type "Vector Structure"))
  (bind _returnvalue (`SceneComponent.K2_GetComponentLocation` self2))
  (if (>= (`local.Alpha`) 1.0)
    (return)
    (else
      (`|ExecutionSequence`
        (:`then_0`
          (`/Engine/EditorBlueprintResources/StandardMacros.DoOnce` false
            (:`Completed`
              (bind _output_get (set `local.StartSize` (+ _returnvalue (`KismetMathLibrary.MakeVector` 0.0 0.0 FallHeight))))
              (set `local.TargetSize` (- _returnvalue (`KismetMathLibrary.MakeVector` 0.0 0.0 FallHeight)))
              (`SceneComponent.K2_SetWorldLocation` self2 _output_get false false))))
        (:`then_1`
          (set `local.Alpha` (+ (/ (`GameplayStatics.GetWorldDeltaSeconds`) 5.0) (`local.Alpha`)))
          (`SceneComponent.K2_SetWorldLocation` self2 (`|EaseFunction` "ExpoInOut" (`local.Alpha`) _returnvalue (`local.TargetSize`)) true false))))))

(fn `UserConstructionScript`)