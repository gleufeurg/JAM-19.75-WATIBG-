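; BP_Spike is a skill spike actor that grows out after spawning.
; On BeginPlay it shrinks to a sixth of its scale, then a looping timer eases the scale up with ExpoInOut, accumulating world delta seconds until alpha reaches one.
; The target adds twice the world forward vector to the start scale, so the stretch depends on actor rotation.
; The MainSpike hit event is empty.
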(event `self.ReceiveBeginPlay`
  (`self.SetActorScale3D` (/ (`self.GetActorScale3D`) 6.0))
  (set `self.Start_size` (`self.GetActorScale3D`))
  (bind _returnvalue (`KismetSystemLibrary.K2_SetTimerDelegate` (delegate `lerpSize`) 0.01 true)))

(event `lerpSize`
  (bind _start_size (`self.Start_size`))
  (bind _output_get (set `self.Alpha` (+ (`GameplayStatics.GetWorldDeltaSeconds`) (`self.Alpha`))))
  (`self.SetActorScale3D` (`|EaseFunction` "ExpoInOut" (`self.Alpha`) _start_size (+ (* (`self.GetActorForwardVector`) 2.0) _start_size)))
  (if (>= _output_get 1.0)
    (`KismetSystemLibrary.K2_ClearAndInvalidateTimerHandle` (stale `self.ReceiveBeginPlay` _returnvalue))))

(event `self.MainSpike.OnComponentHit`
  (params (HitComponent :type "PrimitiveComponent Object Reference") (OtherActor :type "Actor Object Reference") (OtherComp :type "PrimitiveComponent Object Reference") (NormalImpulse :type "Vector Structure") (Hit :type "HitResult Structure (by ref)")))

(fn `UserConstructionScript`)