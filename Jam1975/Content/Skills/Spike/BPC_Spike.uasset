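; Skill component for the first-person character that spawns a BP_Spike on the surface the player is aiming at.
; Target sphere-traces on the Camera channel from the first-person camera, using configurable range and radius.
; UseSkill skips missed traces and hits on existing spikes or BP_Wall actors, otherwise spawning the spike aligned to the impact normal, adjusting for collisions but always spawning.
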(event `self.Use Skill`
  (bind _outhit (`self.Target`))
  (bind (_bblockinghit _binitialoverlap _time _distance _location _impactpoint _normal _impactnormal _physmat _hitactor) (`GameplayStatics.BreakHitResult` _outhit))
  (bind _returnvalue (`GameplayStatics.GetObjectClass` _hitactor))
  (if (not (or (== _returnvalue "/Game/Skills/Spike/BP_Spike.BP_Spike_C") (== _returnvalue "/Game/Skills/Wall/BP_Wall.BP_Wall_C")))
    (`/Engine/EditorBlueprintResources/StandardMacros.IsValid` _hitactor
      (:`Is Valid`
        (`|SpawnActorFromClass` "/Game/Skills/Spike/BP_Spike.BP_Spike_C" (`KismetMathLibrary.MakeTransform` _location (`KismetMathLibrary.Conv_VectorToRotator` _impactnormal)) "AdjustIfPossibleButAlwaysSpawn" "MultiplyWithRoot" null null)))))

(fn `Target`
  (returns (OutHit :type "HitResult Structure"))
  (bind _asbp_first_person_character (cast `/Game/FirstPerson/Blueprints/BP_FirstPersonCharacter` (`self.GetOwner`)))
  (bind _firstpersoncamera (`/Game/FirstPerson/Blueprints/BP_FirstPersonCharacter.FirstPersonCamera` _asbp_first_person_character))
  (bind _returnvalue (`SceneComponent.K2_GetComponentLocation` _firstpersoncamera))
  (bind _outhit (`KismetSystemLibrary.SphereTraceSingle` _returnvalue (+ _returnvalue (* (`SceneComponent.GetForwardVector` _firstpersoncamera) (`self.Targetting Range`))) (`self.Targetting Radius`) "TraceTypeQuery2"))
  (return _outhit))